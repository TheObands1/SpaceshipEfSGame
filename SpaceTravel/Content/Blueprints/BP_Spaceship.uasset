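; Spaceship Blueprint that creates the HUD widget on BeginPlay and handles landing orientation on planets, working around C++ landing logic noted as broken.
; Land builds a rotator from the outward direction of the current planet and the mesh's right vector, keeping only roll.
; It sets that roll instantly, choosing the sign by the ship's Y position, with pitch and yaw zeroed.
; An unused timeline-based rotation remains, marked for removal.
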(event `self.ReceiveBeginPlay`
  (bind _returnvalue (`|CreateWidget` "/Game/Widgets/W_HUD.W_HUD_C"))
  (`UserWidget.AddToViewport` _returnvalue 0))

(event `self.ReceiveTick`
  (params (DeltaSeconds :type "Float (single-precision)")))

(event `self.BP_Land`
  (bind (_returnvalue_x _returnvalue_y) (`KismetMathLibrary.BreakVector` (`self.K2_GetActorLocation`)))
  (bind _returnvalue_roll (`KismetMathLibrary.BreakRotator` (`KismetMathLibrary.MakeRotFromZY` (`KismetMathLibrary.GetForwardVector` (`KismetMathLibrary.FindLookAtRotation` (`self.K2_GetActorLocation` (`self.CurrentPlanetReference`)) (`self.K2_GetActorLocation`))) (`SceneComponent.GetRightVector` (`self.SpaceshipMeshComponent`)))))
  ;[1 1 1] Landing Behavior. It is programmed in c++, yet it does not work there
  (set `self.BP_RotatorFromZY` _returnvalue_roll)
  (if (< _returnvalue_y 0.0)
    (if (< (`self.BP_RotatorFromZY`) 0.0)
      (`self.K2_SetActorRotation` (`KismetMathLibrary.MakeRotator` (`self.BP_RotatorFromZY`)))
      (else
        (`self.K2_SetActorRotation` (`KismetMathLibrary.MakeRotator` (* (`self.BP_RotatorFromZY`) -1.0)))))
    (else
      (`self.K2_SetActorRotation` (`KismetMathLibrary.MakeRotator` (`KismetMathLibrary.Abs` (`self.BP_RotatorFromZY`)))))))

(fn `UserConstructionScript`)